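; Guard AI pawn that detects the player by sight and passes that awareness to its behavior tree Blackboard.
; PawnSensing sightings set the seen and in-sight flags, store the player's last location in a variable, and write the player reference.
; A retriggerable delay clears only the in-sight flag once ChasingTimeout passes without another sighting.
; Tick separately counts the high-alert timer down to zero.
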(event OnSeePawn(PawnSensing)
  (params (Pawn :type Pawn%20Object%20Reference))
  (bind _returnvalue (Utilities|Name|MakeLiteralName "playerInSight"))
  (bind _self self)
  (bind _returnvalue_2 (AI|GetAIController _self))
  (bind _returnvalue_3 (AI|GetBlackboard _returnvalue_2))
  (bind _asplayer_character (Utilities|Casting|CastToPlayerCharacter Pawn))
  (Utilities|FlowControl|Sequence
    (:then_0
      (AI|Components|Blackboard|SetValueasBool _returnvalue_3 (Utilities|Name|MakeLiteralName "hasSeenPlayer") true)
      (AI|Components|Blackboard|SetValueasBool _returnvalue_3 _returnvalue true)
      (Variables|Default|SetLast%20Seen%20Location (Transformation|GetActorLocation _asplayer_character))
      (AI|Components|Blackboard|SetValueasObject _returnvalue_3 (Utilities|Name|MakeLiteralName "player") (Game|Player|GetPlayerPawn 0)))
    (:then_1
      (Utilities|FlowControl|RetriggerableDelay (Variables|Default|GetChasing%20Timeout))
      (AI|Components|Blackboard|SetValueasBool _returnvalue_3 _returnvalue false))))

(event EventTick
  (params (DeltaSeconds :type Float%20%28single-precision%29))
  (if (>= (- (Variables|Default|GetCurrent%20High%20Alert%20Timeout) DeltaSeconds) 0.0)
    (Variables|Default|SetCurrent%20High%20Alert%20Timeout (- (Variables|Default|GetCurrent%20High%20Alert%20Timeout) DeltaSeconds))
    (else
      (Variables|Default|SetCurrent%20High%20Alert%20Timeout 0.0))))

(fn ConstructionScript)